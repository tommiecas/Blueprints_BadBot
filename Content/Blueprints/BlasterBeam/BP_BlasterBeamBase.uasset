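; BP_BlasterBeamBase is a base blaster beam actor that deals damage and destroys itself on impact.
; On BeginPlay it binds to BeamMesh's component hit event, which passes the hit and the beam's effect and damage values to HandleOnHitToDieOrToQuit.
; That function spawns the impact effect oriented to the hit normal, sends GetHurtMessage to actors implementing BPI_Damageable, then destroys the beam.
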(event Custom|OnComponentHit_Event
  (params (HitComponent :type Primitive%20Component%20Object%20Reference) (OtherActor :type Actor%20Object%20Reference) (OtherComp :type Primitive%20Component%20Object%20Reference) (NormalImpulse :type Vector) (Hit :type Hit%20Result%20Structure%20%28by%20ref%29))
  (CallFunction|HandleonHittoDieortoQuit OtherActor Hit (Variables|Default|GetParticleSystem) (Variables|Default|GetDamage)))

(event EventBeginPlay
  (Collision|AssignOnComponentHit (Variables|Default|GetBeamMesh) (delegate Custom|OnComponentHit_Event)))

(event Collision|EventActorBeginOverlap
  (params (OtherActor :type Actor%20Object%20Reference)))

(event EventTick
  (params (DeltaSeconds :type Float%20%28single-precision%29)))

(fn ConstructionScript)

(fn HandleonHittoDieortoQuit
  (params (TheActorHit :type Actor%20Object%20Reference) (Hit :type Hit%20Result%20Structure%20%28by%20ref%29) (ExplosionEffects :type Niagara%20System%20Object%20Reference) (Damage :type Float%20%28double-precision%29))
  (bind (_bblockinghit _binitialoverlap _time _distance _location _impactpoint _normal) (Collision|BreakHitResult Hit))
  (Niagara|SpawnSystematLocation ExplosionEffects _impactpoint (Math|Rotator|MakeRotfromX _normal))
  (if (Utilities|DoesObjectImplementInterface TheActorHit "/Game/Blueprints/Interfaces/BPI_Damageable.BPI_Damageable_C")
    (Class|BPIDamageable|GetHurt(Message) TheActorHit Damage))
  (Actor|DestroyActor))