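; BP_FloatingSphere is a collectible sphere that awards score through BP_BadBotGameMode when a DefaultPawn overlaps it.
; After a short delay it scales in by timeline, picks a random rotation delta, starts a lifetime timer and binds the overlap.
; Timer expiry or pickup triggers a guarded wink-out timeline that shrinks and destroys it.
; Tick calls UpdateLocation and UpdateRotation, but both are empty here, leaving the rotation delta unused.
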(event Custom|WinkOut
  ;[0 0.1046 0.15 0.5] Spheres "Wink-Out"
  (if (not (Variables|Default|GetIsWinking))
    (Variables|Default|SetIsWinking true)
    (bind _scale (Timeline|WinkOutTimeline Play)
      (:Update
        (CallFunction|SetWorldScale _scale))
      (:Finished
        (Actor|DestroyActor)))))

(event Custom|WinkIn
  (bind _scale (Timeline|WinkInTimeline Play)
    (:Update
      (Transformation|SetWorldScale3D (Variables|Default|GetSphereMesh) _scale))))

(event Custom|OnComponentBeginOverlap_Event
  (params (OverlappedComponent :type Primitive%20Component%20Object%20Reference) (OtherActor :type Actor%20Object%20Reference) (OtherComp :type Primitive%20Component%20Object%20Reference) (OtherBodyIndex :type Integer) (bFromSweep :type Boolean) (SweepResult :type Hit%20Result%20Structure%20%28by%20ref%29))
  ;[0.15 0.04324 0.09946 0.5] Handle Overlap
  (if (Class|GameplayStatics|ObjectIsA OtherActor "/Script/Engine.DefaultPawn")
    (bind _asbp_bad_bot_game_mode (Utilities|Casting|CastToBP_BadBotGameMode (Game|GetGameMode)))
    (Default|IncrementScore _asbp_bad_bot_game_mode)
    (CallFunction|WinkOut)))

(event EventBeginPlay
  (Utilities|FlowControl|Delay 2.0)
  (CallFunction|Winkin)
  (CallFunction|InitializeDeltaRotation)
  ;[0 0.1046 0.15 0.5] Spheres "Wink-Out"
  (Utilities|Time|SetTimerbyEvent (delegate Custom|WinkOut) (Variables|Default|GetSphereLifetime))
  ;[0.15 0.04324 0.09946 0.5] Handle Overlap
  (Collision|AssignOnComponentBeginOverlap (Variables|Default|GetSphereCollision) (delegate Custom|OnComponentBeginOverlap_Event)))

(event EventTick
  (params (DeltaSeconds :type Float%20%28single-precision%29))
  ;[0.1695 1 0] Update Location and Rotation
  (CallFunction|UpdateLocation DeltaSeconds)
  (CallFunction|UpdateRotation DeltaSeconds))

(fn ConstructionScript)

(fn InitializeDeltaRotation
  (Variables|Default|SetDeltaRotation (* (Math|Random|RandomRotator false) (Variables|Default|GetRotationScaleFactor))))

(fn UpdateLocation
  (params (DeltaTime :type Float%20%28double-precision%29)))

(fn UpdateRotation
  (params (DeltaTime :type Float%20%28single-precision%29)))

(fn SetWorldScale
  (params (Scale%20Winking%20Out :type Float%20%28single-precision%29))
  (Transformation|SetWorldScale3D (Variables|Default|GetSphereMesh) (Math|Vector|MakeVector Scale%20Winking%20Out Scale%20Winking%20Out Scale%20Winking%20Out)))