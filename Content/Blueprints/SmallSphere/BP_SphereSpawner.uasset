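; BP_SphereSpawner is an actor that continually spawns BP_FloatingSphere actors at random points around itself.
; BeginPlay starts a looping timer at SpawnTime intervals, and each firing spawns one sphere with a random rotation.
; GetRandomPointWithinSphereRadius picks each location by scaling a random rotator's forward vector by a random distance up to SpawnRadius, offset from the spawner's location.
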(event Custom|SpawnSmallSphere
  ;[0.09695 0 0.15 0.5] Start Sphere Spawn Timer
  (Game|SpawnActorfromClass "/Game/Blueprints/SmallSphere/BP_FloatingSphere.BP_FloatingSphere_C" (Math|Transform|MakeTransform (CallFunction|GetRandomPointWithinSphereRadius) (Math|Random|RandomRotator false) "1.000000,1.000000,1.000000") "Undefined" "MultiplyWithRoot" 0 0))

(event EventBeginPlay
  ;[0.09695 0 0.15 0.5] Start Sphere Spawn Timer
  (Utilities|Time|SetTimerbyEvent (delegate Custom|SpawnSmallSphere) (Variables|Default|GetSpawnTime) true))

(event EventTick
  (params (DeltaSeconds :type Float%20%28single-precision%29)))

(fn ConstructionScript)

(fn GetRandomPointWithinSphereRadius
  (return (+ (Transformation|GetActorLocation) (* (Math|Vector|GetForwardVector (Math|Random|RandomRotator false)) (Math|Random|RandomFloatinRange (Variables|SphereSpawner|GetSpawnRadius) 0.0)))))